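; Character inventory component that tracks a character's guns and the slots used to equip and switch between them.
; GunSlots holds indices into the gun inventory, with -1 for empty; new guns fill the first free slot.
; Pickups are two-phase: PreAdd counts a pending pickup against capacity, FinishAdd releases it and stores the gun.
; Switching stops the current gun, assigns the owning CharacterBaseClass to the new one and updates its sprite.
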(event EventTick
  (params (DeltaSeconds :type Float%20%28single-precision%29)))

(event EventBeginPlay)

(fn IsInventoryFull
  (bind _size (CallFunction|GetCurrentInventorySize))
  (return (>= (+ _size (Variables|Default|GetcurrentPickupCount)) (Variables|Default|GetinventorySize))))

(fn PreAddtoInventory
  (bind _isfull (CallFunction|IsInventoryFull))
  (if _isfull
    (return false)
    (else
      (bind _result (Math|Integer|IncrementInt (Variables|Default|GetcurrentPickupCount))
        (:%20%20
          (return (< _result (Variables|Default|GetinventorySize))))))))

(fn FinishAddtoInventory
  (params (gun :type Gun%20Base%20Class%20Object%20Reference) (isJunk :type Boolean))
  (Math|Integer|DecrementInt (Variables|Default|GetcurrentPickupCount)
    (:%20%20
      (bind (_success _index) (CallFunction|AddGuntoInventory gun isJunk))
      (for _index_2 (range 0 (- (Variables|GunSlots|GetnumberOfGunSlots) 1))
        (if (== (Utilities|Array|Get(acopy) (Variables|GunSlots|GetgunSlots) _index_2) -1)
          (GunSlots|SetGunbySlot _index_2 _index)
          (return _success _index)))
      (return _success _index))))

(fn GetCurrentGun
  (bind _gunslots (Variables|GunSlots|GetgunSlots))
  (bind _curentgunslot (Variables|GunSlots|GetcurentGunSlot))
  (bind _item (Utilities|Array|Get(acopy) _gunslots _curentgunslot))
  (Math|Integer|CompareInt _item -1
    (:>
      (bind _gun (CallFunction|GetGunfromIndex _item))
      (bind _output_get (LocalVariables|SetgunToReturn _gun))
      (LocalVariables|Setsuccess (Utilities|IsValid _output_get)))
    (:==
      (LocalVariables|Setsuccess false :!label _label))
    (:<
      (goto _label)))
  (return (LocalVariables|Getsuccess) (LocalVariables|GetgunToReturn) _item))

(fn SwitchGuns
  (params (gunSlotToSwitchTo :type Integer))
  ;[1 1 1] Check slot is within range
  (bind _output_get (LocalVariables|SetgunSlot gunSlotToSwitchTo))
  (Math|Integer|CompareInt _output_get (- (Variables|GunSlots|GetnumberOfGunSlots) 1)
    (:==
      _)
    (:<
      _))
  ;[1 1 1] Make sure slot isn't empty
  (if (!= (Utilities|Array|Get(acopy) (Variables|GunSlots|GetgunSlots) (LocalVariables|GetgunSlot)) -1)
    ;[1 1 1] Stop shooting if currently using a gun
    (bind (_isholdinggun _gun) (GunSlots|GetCurrentGun))
    (if _isholdinggun
      (Default|StopUsingGun _gun))
    (Variables|GunSlots|SetcurentGunSlot (LocalVariables|GetgunSlot))
    (bind _gun_2 (GunSlots|GetCurrentGun))
    (bind _ascharacter_base_class (Utilities|Casting|CastToCharacterBaseClass (Components|GetOwner)))
    (Variables|/Game/Loot/Guns/Blueprints/GunBaseClass.GunBaseClass_C|Setcharacter _gun_2 _ascharacter_base_class)
    (Rendering|Components|Sprite|SetSprite _ascharacter_base_class (Variables|/Game/Loot/Guns/Blueprints/GunBaseClass.GunBaseClass_C|GetgunSprite _gun_2))
    (return)))

(fn SetGunbySlot
  (params (slot :type Integer) (gunIndex :type Integer))
  ;[1 1 1] Setup
  (LocalVariables|Set_slot slot)
  (LocalVariables|Set_gunIndex gunIndex)
  ;[1 1 1] Check if slot is valid
  (if (and (>= (LocalVariables|Get_slot) 0) (<= (LocalVariables|Get_slot) (- (Variables|GunSlots|GetnumberOfGunSlots) 1)))
    ;[1 1 1] Check if gun index is valid
    (if (and (>= (LocalVariables|Get_gunIndex) 0) (<= (LocalVariables|Get_gunIndex) (- (Variables|Default|GetinventorySize) 1)))
      ;[1 1 1] Update gun slots
      (Utilities|Array|SetArrayElem (Variables|GunSlots|GetgunSlots) (LocalVariables|Get_slot) (LocalVariables|Get_gunIndex))
      ;[1 1 1] Check if current gun is updated
      (if (== (Variables|GunSlots|GetcurentGunSlot) (LocalVariables|Get_slot))
        (GunSlots|SwitchGuns (LocalVariables|Get_slot)))
      ;[1 1 1] Returns
      (LocalVariables|SetreturnValue false)
      (else
        (bind _output_get (LocalVariables|SetreturnValue false :!label _label))))
    (else
      (goto _label)))
  (return _output_get))

(fn ChangeNumberOfGunSlots
  (params (newNumberOfGunSlots :type Integer))
  (bind _output_get (LocalVariables|SettempNewNumberOfGunSlots newNumberOfGunSlots))
  (Math|Integer|CompareInt _output_get (Variables|GunSlots|GetnumberOfGunSlots)
    (:>
      (for _index (range (- (Variables|GunSlots|GetnumberOfGunSlots) 1) (- (LocalVariables|GettempNewNumberOfGunSlots) 1))
        (Utilities|Array|Add (Variables|GunSlots|GetgunSlots) -1)))
    (:<
      (for _index_2 (range (- (LocalVariables|GettempNewNumberOfGunSlots) 1) (- (Variables|GunSlots|GetnumberOfGunSlots) 1))
        (Utilities|Array|RemoveIndex (Variables|GunSlots|GetgunSlots) _index_2))))
  (bind _output_get_2 (Variables|GunSlots|SetnumberOfGunSlots (LocalVariables|GettempNewNumberOfGunSlots)))
  (if (> (Variables|GunSlots|GetcurentGunSlot) _output_get_2)
    ;[1 1 1] prevent null pointer
    (Variables|GunSlots|SetcurentGunSlot 0)
    (GunSlots|SwitchGuns)))

(fn AddGunSlot
  (GunSlots|ChangeNumberOfGunSlots (+ (Variables|GunSlots|GetnumberOfGunSlots) 1)))

(fn ClearSlot
  (params (slotToClear :type Integer))
  (Utilities|Array|SetArrayElem (Variables|GunSlots|GetgunSlots) slotToClear -1)
  (if (== slotToClear (Variables|GunSlots|GetcurentGunSlot))
    (bind _index (Utilities|FlowControl|ForLoopwithBreak 0 (Variables|GunSlots|GetnumberOfGunSlots))
      (:LoopBody
        (if (!= (Utilities|Array|Get(acopy) (Variables|GunSlots|GetgunSlots) _index) -1)
          (GunSlots|SwitchGuns _index)
          (return)))
      (:Completed
        ;[1 1 1] No gun, clear sprite
        (GunSlots|SwitchGuns (Variables|GunSlots|GetcurentGunSlot))))))

(fn GetSlotbyGunIndex
  (params (gunIndex :type Integer))
  (return (Utilities|Array|FindItem (Variables|GunSlots|GetgunSlots) gunIndex)))

(fn GetCurrentGunSlot
  (return (Variables|GunSlots|GetcurentGunSlot)))