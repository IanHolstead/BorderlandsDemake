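; Character inventory Blueprint that stores guns up to a size limit, with a parallel array flagging each as junk.
; Adding is two-phase: TestAddToInventory reserves space by incrementing a pending-pickup count, which IsInventoryFull counts alongside stored guns.
; FinishAddToInventory releases the reservation, rechecks capacity, then appends the gun and junk flag, returning the new index.
; Its Sucess output carries the InventoryFull value, so it is false on a successful add.
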(event EventTick
  (params (DeltaSeconds :type Float%20%28single-precision%29)))

(event EventInitializeComponent)

(fn IsInventoryFull
  (return (>= (+ (Utilities|Array|Length (Variables|Default|Getguns)) (Variables|Default|GetcurrentPickupCount)) (Variables|Default|GetinventorySize))))

(fn TestAddtoInventory
  (bind _isfull (CallFunction|IsInventoryFull))
  (if (not _isfull)
    (bind _output_get (Variables|Default|SetcurrentPickupCount (+ (Variables|Default|GetcurrentPickupCount) 1)))
    (return (< _output_get (Variables|Default|GetinventorySize)))))

(fn FinishAddtoInventory
  (params (gun :type Gun%20Base%20Class%20Object%20Reference) (isJunk :type Boolean))
  (LocalVariables|SetincomingGun gun)
  (LocalVariables|SetisIncomingJunk isJunk)
  (Variables|Default|SetcurrentPickupCount (- (Variables|Default|GetcurrentPickupCount) 1))
  ;[1 1 1] This shouldn't be needed, it should never fail
  (bind _isfull (CallFunction|IsInventoryFull))
  (bind _output_get (LocalVariables|SetinventoryFull _isfull))
  (if (not _output_get)
    (Utilities|Array|Add (Variables|Default|Getguns) (LocalVariables|GetincomingGun))
    (bind _returnvalue (Utilities|Array|Add (Variables|Default|GetisJunk) (LocalVariables|GetisIncomingJunk)))
    (return (LocalVariables|GetinventoryFull) _returnvalue)))