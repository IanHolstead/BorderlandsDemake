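; Profile list save loader that returns the saved player profiles and guests from two save slots.
; LoadProfiles handles the guest slot then the profile slot, loading each ProfileList save or creating and saving a new one when absent.
; A failed cast of a loaded save prints an error.
; An existing guest save is assigned to ProfileSave, not GuestSave, and is then overwritten by the profile save.
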(fn LoadProfiles
  (bind _returnvalue (SaveGame|DoesSaveGameExist (Utilities|GuestSlot)))
  (if _returnvalue
    (bind _returnvalue_2 (SaveGame|LoadGamefromSlot (Utilities|GuestSlot)))
    (bind _asprofile_list (Utilities|Casting|CastToProfileList _returnvalue_2)
      (:then
        (LocalVariables|SetprofileSave _asprofile_list)
        (bind _returnvalue_3 (SaveGame|DoesSaveGameExist (Utilities|ProfileSlot) :!label _label))
        (if _returnvalue_3
          (bind _returnvalue_4 (SaveGame|LoadGamefromSlot (Utilities|ProfileSlot)))
          (bind _asprofile_list_2 (Utilities|Casting|CastToProfileList _returnvalue_4)
            (:then
              (LocalVariables|SetprofileSave _asprofile_list_2)
              (return (Variables|ProfileList_C|Getprofiles (LocalVariables|GetprofileSave)) (Variables|ProfileList_C|Getprofiles (LocalVariables|GetguestSave))))
            (:CastFailed
              (Utilities|PrintError _returnvalue_4)))
          (else
            (bind _returnvalue_5 (SaveGame|CreateSaveGameObject "ProfileList_C"))
            (bind _asprofile_list_3 (Utilities|Casting|CastToProfileList _returnvalue_5))
            (bind _output_get (LocalVariables|SetprofileSave _asprofile_list_3))
            (SaveGame|SaveGametoSlot _output_get (Utilities|ProfileSlot))
            (return (Variables|ProfileList_C|Getprofiles (LocalVariables|GetprofileSave)) (Variables|ProfileList_C|Getprofiles (LocalVariables|GetguestSave))))))
      (:CastFailed
        (Utilities|PrintError _returnvalue_2)))
    (else
      (bind _returnvalue_6 (SaveGame|CreateSaveGameObject "ProfileList_C"))
      (bind _asprofile_list_4 (Utilities|Casting|CastToProfileList _returnvalue_6))
      (bind _output_get_2 (LocalVariables|SetguestSave _asprofile_list_4))
      (SaveGame|SaveGametoSlot _output_get_2 (Utilities|GuestSlot))
      (goto _label))))