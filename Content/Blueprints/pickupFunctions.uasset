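; A pickup helper function that removes a given actor from the pickup stack of each character overlapping its collision shape.
; It accepts sphere, box and capsule components, checks which is set, and gathers the overlapping CharacterBaseClass actors from it.
; Each gathered character is cast to CharacterBaseClass and told to remove the actor from its stack.
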(fn RemovefromPickupStacks
  (params (SphereCollisionComponent :type Sphere%20Component%20Object%20Reference) (BoxCollisionComponent :type Box%20Component%20Object%20Reference) (CapsuleCollisionComponent :type Capsule%20Component%20Object%20Reference) (actorToRemove :type Actor%20Object%20Reference))
  ;[1 1 1] There will only be one collision component used, but we have to check which one and use it without using the others
  (LocalVariables|Setsphere SphereCollisionComponent)
  (LocalVariables|Setbox BoxCollisionComponent)
  (LocalVariables|Setcapsule CapsuleCollisionComponent)
  (if (== (LocalVariables|Getsphere) 0)
    _
    (else
      (Utilities|Array|AppendArray (LocalVariables|Getactors) (Collision|GetOverlappingActors (LocalVariables|Getsphere) "/Game/Characters/Blueprints/CharacterBaseClass.CharacterBaseClass_C" :!class /Script/Engine.PrimitiveComponent))))
  (if (== (LocalVariables|Getbox) 0)
    _
    (else
      (Utilities|Array|AppendArray (LocalVariables|Getactors) (Collision|GetOverlappingActors (LocalVariables|Getbox) "/Game/Characters/Blueprints/CharacterBaseClass.CharacterBaseClass_C" :!class /Script/Engine.PrimitiveComponent))))
  (if (== (LocalVariables|Getcapsule) 0)
    _
    (else
      (Utilities|Array|AppendArray (LocalVariables|Getactors) (Collision|GetOverlappingActors (LocalVariables|Getcapsule) "/Game/Characters/Blueprints/CharacterBaseClass.CharacterBaseClass_C" :!class /Script/Engine.PrimitiveComponent))))
  (for _array_element (LocalVariables|Getactors)
    (bind _ascharacter_base_class (Utilities|Casting|CastToCharacterBaseClass _array_element))
    (Default|RemovefromPickupStack _ascharacter_base_class actorToRemove)))