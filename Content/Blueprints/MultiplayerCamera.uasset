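; Multiplayer side-on orthographic camera actor that follows a list of registered actors and moves Left and Right walls with its view.
; Each tick while following, it scans actor X and Z positions to recenter the camera and set a clamped ortho width from the padded X spread.
; The walls teleport to the view's horizontal edges, and UpdateWallCollision toggles their collision to match the follow flag.
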(event EventBeginPlay
  (Transformation|SetActorRotation "0,-90.000000, 0"))

(event EventTick
  (params (DeltaSeconds :type Float%20%28single-precision%29))
  (if (Variables|Default|GetisFollowingCamera)
    (CallFunction|UpdateWallPosition)))

(fn ConstructionScript)

(fn UpdateWallPosition
  (bind _actors_to_follow (Variables|Default|GetActors%20to%20Follow))
  (bind _actors_to_follow_2 (Variables|Default|GetActors%20to%20Follow))
  (bind _item (Utilities|Array|Get(acopy) _actors_to_follow_2))
  (bind _returnvalue (Transformation|GetActorLocation _item))
  (bind (_x _y _z) (Math|Vector|BreakVector _returnvalue))
  (bind _output_get (LocalVariables|SetMaxXPos _x))
  (LocalVariables|SetMinXPos _output_get)
  (bind _output_get_2 (LocalVariables|SetMaxZPos _z))
  (LocalVariables|SetMinZPos _output_get_2)
  (LocalVariables|SetactorCount (Utilities|Array|Length _actors_to_follow))
  (for _array_element _actors_to_follow
    (Math|Float|CompareFloat (LocalVariables|GetMinXPos) (.X (Math|Vector|BreakVector (.Location (Math|Transform|BreakTransform (Transformation|GetActorTransform _array_element)))))
      (:>
        (LocalVariables|SetMinXPos (.X (Math|Vector|BreakVector (.Location (Math|Transform|BreakTransform (Transformation|GetActorTransform _array_element)))))))
      (:==
        _)
      (:<
        _))
    (Math|Float|CompareFloat (.X (Math|Vector|BreakVector (.Location (Math|Transform|BreakTransform (Transformation|GetActorTransform _array_element))))) (LocalVariables|GetMaxXPos)
      (:>
        (LocalVariables|SetMaxXPos (.X (Math|Vector|BreakVector (.Location (Math|Transform|BreakTransform (Transformation|GetActorTransform _array_element)))))))
      (:==
        _)
      (:<
        _))
    (Math|Float|CompareFloat (LocalVariables|GetMinZPos) 0.0
      (:>
        (LocalVariables|SetMinZPos (.Z (Math|Vector|BreakVector (.Location (Math|Transform|BreakTransform (Transformation|GetActorTransform _array_element)))))))
      (:==
        _)
      (:<
        _))
    (Math|Float|CompareFloat (.Z (Math|Vector|BreakVector (.Location (Math|Transform|BreakTransform (Transformation|GetActorTransform _array_element))))) (LocalVariables|GetMaxZPos)
      (:>
        (LocalVariables|SetMinZPos (.Z (Math|Vector|BreakVector (.Location (Math|Transform|BreakTransform (Transformation|GetActorTransform _array_element)))))))))
  (Variables|/Script/Engine.CameraComponent|SetOrthoWidth (Variables|CameraActor|GetCameraComponent) (Math|Float|Clamp(Float) (- (+ (LocalVariables|GetMaxXPos) 2e+02) (- (LocalVariables|GetMinXPos) 2e+02)) (Variables|Default|GetminWidth) (Variables|Default|GetmaxWidth)))
  (Transformation|SetWorldLocation (Variables|CameraActor|GetCameraComponent) (Math|Vector|MakeVector (/ (+ (LocalVariables|GetMaxXPos) (LocalVariables|GetMinXPos)) 2.0) 0.0 (/ (+ (LocalVariables|GetMaxZPos) (LocalVariables|GetMinZPos)) 2.0)) false false)
  (Transformation|SetWorldLocation (Variables|Default|GetLeft) (- (Math|Vector|MakeVector (/ (+ (LocalVariables|GetMaxXPos) (LocalVariables|GetMinXPos)) 2.0) 0.0 (/ (+ (LocalVariables|GetMaxZPos) (LocalVariables|GetMinZPos)) 2.0)) (Math|Vector|MakeVector (/ (Variables|/Script/Engine.CameraComponent|GetOrthoWidth (Variables|CameraActor|GetCameraComponent)) 2.0) 0.0 0.0)) false true)
  (Transformation|SetWorldLocation (Variables|Default|GetRight) (+ (Math|Vector|MakeVector (/ (+ (LocalVariables|GetMaxXPos) (LocalVariables|GetMinXPos)) 2.0) 0.0 (/ (+ (LocalVariables|GetMaxZPos) (LocalVariables|GetMinZPos)) 2.0)) (Math|Vector|MakeVector (/ (Variables|/Script/Engine.CameraComponent|GetOrthoWidth (Variables|CameraActor|GetCameraComponent)) 2.0) 0.0 0.0)) false true))

(fn UpdateWallCollision
  (if (Variables|Default|GetisFollowingCamera)
    (Collision|SetCollisionEnabled (Variables|Default|GetRight) "QueryAndPhysics")
    (Collision|SetCollisionEnabled (Variables|Default|GetLeft) "QueryAndPhysics")
    (else
      (Collision|SetCollisionEnabled (Variables|Default|GetRight) "NoCollision")
      (Collision|SetCollisionEnabled (Variables|Default|GetLeft) "NoCollision"))))

(fn AddActortoFollow
  (params (ActorToFollow :type Actor%20Object%20Reference))
  (Utilities|Array|AddUnique (Variables|Default|GetActors%20to%20Follow) ActorToFollow))

(fn RemoveActor
  (params (ActorToRemove :type Actor%20Object%20Reference))
  (Utilities|Array|RemoveItem (Variables|Default|GetActors%20to%20Follow) ActorToRemove))