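; RespawnStation is a level actor that spawns player characters.
; Its respawn event spawns a TestCharacter at the station's transform and has the supplied controller possess it.
; Pressing 0 spawns a new TestPlayerController and a TestCharacter at a game mode player start, possesses it, then registers the character with the camera held in myGameInstance to follow.
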(event Custom|respawn
  (params (controller :type Player%20Controller%20Object%20Reference))
  (bind _returnvalue (Game|SpawnActorfromClass "/Game/Characters/Blueprints/testCharacter.testCharacter_C" (Transformation|GetActorTransform) "Undefined" 0 0))
  (Pawn|Possess controller _returnvalue))

(event EventBeginPlay)

(event EventActorBeginOverlap
  (params (OtherActor :type Actor%20Object%20Reference)))

(event EventTick
  (params (DeltaSeconds :type Float%20%28single-precision%29)))

(event Input|KeyboardEvents|0
  (params (Key :type Key%20Structure :default "AnyKey"))
  (:Pressed
    (bind _returnvalue (Game|SpawnActorfromClass "/Game/Characters/Blueprints/testPlayerController.testPlayerController_C" (Math|Transform|MakeTransform "0, 0, 0") "Undefined" 0 0))
    (bind _returnvalue_2 (Game|SpawnActorfromClass "/Game/Characters/Blueprints/testCharacter.testCharacter_C" (Math|Conversions|ToTransform(Vector) (Transformation|GetActorLocation (Class|GameMode|FindPlayerStart (Game|GetGameMode) _returnvalue))) "Undefined" 0 0))
    (Pawn|Possess _returnvalue _returnvalue_2)
    (bind _asmy_game_instance (Utilities|Casting|CastTomyGameInstance (Game|GetGameInstance)))
    (Default|AddActortoFollow (Variables|/Game/Blueprints/myGameInstance.myGameInstance_C|Getcamera _asmy_game_instance) _returnvalue_2)))

(fn ConstructionScript)