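; Level helper functions that set up a shared follow camera and spawn player characters.
; SetupCamera stores the camera in myGameInstance, makes it follow the controller's pawn and sets it as that controller's view target.
; SpawnPlayer spawns a TestPlayerController and a TestCharacter at the given location, possesses the character and adds it to the stored camera's followed actors.
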(fn SetupCamera
  (params (camera :type Multiplayer%20Camera%20Object%20Reference) (gameInstance :type Game%20Instance%20Object%20Reference) (playerController :type Player%20Controller%20Object%20Reference))
  (bind _asmy_game_instance (Utilities|Casting|CastTomyGameInstance gameInstance))
  (bind _output_get (Variables|/Game/Blueprints/myGameInstance.myGameInstance_C|Setcamera _asmy_game_instance camera))
  (Default|AddActortoFollow _output_get (Pawn|GetControlledPawn playerController))
  (Game|Player|SetViewTargetwithBlend playerController _output_get 0.0 "VTBlend_Linear" 0.0 false))

(fn SpawnPlayer
  (params (location :type Vector) (gameInstance :type Game%20Instance%20Object%20Reference))
  (bind _returnvalue (Game|SpawnActorfromClass "/Game/Characters/Blueprints/testPlayerController.testPlayerController_C" (Math|Transform|MakeTransform "0, 0, 0") "Undefined" 0 0))
  (bind _returnvalue_2 (Game|SpawnActorfromClass "/Game/Characters/Blueprints/testCharacter.testCharacter_C" (Math|Conversions|ToTransform(Vector) location) "Undefined" 0 0))
  (Pawn|Possess _returnvalue _returnvalue_2)
  (bind _asmy_game_instance (Utilities|Casting|CastTomyGameInstance gameInstance))
  (Default|AddActortoFollow (Variables|/Game/Blueprints/myGameInstance.myGameInstance_C|Getcamera _asmy_game_instance) _returnvalue_2))