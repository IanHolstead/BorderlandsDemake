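; Usable chest actor that spawns a random gun once opened.
; Its Box overlap adds or removes it from a character's pickup stack, and Use removes it from pickup stacks and destroys a component to prevent reuse.
; A timeline fades the sprite from green to grey, then spawns a gun from the game instance's GunList above it with physics simulation off.
; GetPointerLocation supplies a point above the sprite.
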(event OnComponentBeginOverlap(Box)
  (params (OtherActor :type Actor%20Object%20Reference) (OtherComp :type Primitive%20Component%20Object%20Reference) (OtherBodyIndex :type Integer) (bFromSweep :type Boolean) (SweepResult :type Hit%20Result%20Structure%20%28by%20ref%29))
  ;[1 1 1] Add to pickup stacks when actor overlaps
  (bind _ascharacter_base_class (Utilities|Casting|CastToCharacterBaseClass OtherActor))
  (Default|AddtoPickupStack _ascharacter_base_class self))

(event OnComponentEndOverlap(Box)
  (params (OtherActor :type Actor%20Object%20Reference) (OtherComp :type Primitive%20Component%20Object%20Reference) (OtherBodyIndex :type Integer))
  ;[1 1 1] Remove from pickup stacks when overlap ends
  (bind _ascharacter_base_class (Utilities|Casting|CastToCharacterBaseClass OtherActor))
  (Default|RemovefromPickupStack _ascharacter_base_class self))

(event EventUse
  (params (user :type Character%20Base%20Class%20Object%20Reference) (secondUse :type Boolean))
  ;[1 1 1] Use
  ;;[1 1 1] make sure no one uses again
  (CallFunction|RemovefromPickupStacks 0 (Variables|Default|GetBox) 0 self)
  (Components|DestroyComponent)
  ;;[1 1 1] Open chest
  (bind _lightalpha (Timeline|lightcolour PlayFromStart)
    (:Update
      (Sprite|SetSpriteColor (Math|Color|Lerp(LinearColor) "(R=0.000000,G=1.000000,B=0.000000,A=1.000000)" "(R=0.675000,G=0.675000,B=0.675000,A=1.000000)" _lightalpha)))
    (:Finished
      (bind _asmy_game_instance (Utilities|Casting|CastTomyGameInstance (Game|GetGameInstance)))
      (bind _returnvalue (Game|SpawnActorfromClass (Utilities|Array|Get(acopy) (Variables|/Game/Blueprints/myGameInstance.myGameInstance_C|GetgunList _asmy_game_instance) (Math|Random|RandomInteger (Utilities|Array|Length (Variables|/Game/Blueprints/myGameInstance.myGameInstance_C|GetgunList _asmy_game_instance)))) (Math|Transform|MakeTransform (+ (Transformation|GetWorldLocation self) "0,0.000000,40.000000")) true 0))
      (Physics|SetSimulatePhysics _returnvalue false))))

(event EventBeginPlay)

(event EventTick
  (params (DeltaSeconds :type Float%20%28single-precision%29)))

(fn ConstructionScript)

(fn GetPointerLocation
  (return (+ (Transformation|GetWorldLocation (Variables|Default|GetPaperSprite)) "0, 0,45.000000")))