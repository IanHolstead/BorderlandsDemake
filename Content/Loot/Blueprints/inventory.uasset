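; Loot inventory Blueprint that stores guns up to InventorySize, each with a junk flag.
; Guns and IsJunk are parallel arrays sharing indices, so adds and removals update both together.
; Adding is gated by a capacity check, and removal rejects indices past the end but never sets Success to true.
; Helper functions read a gun with its flag or change the flag by index.
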(event EventTick
  (params (DeltaSeconds :type Float%20%28single-precision%29)))

(event EventBeginPlay)

(fn AddGuntoInventory
  (params (gun :type Gun%20Base%20Class%20Object%20Reference) (isJunk :type Boolean :default false))
  (LocalVariables|SetincomingGun gun)
  (LocalVariables|SetisIncomingJunk isJunk)
  (bind _isfull (CallFunction|IsInventoryFull))
  (bind _output_get (LocalVariables|SetinventoryFull _isfull))
  (if _output_get
    _
    (else
      (bind _returnvalue (Utilities|Array|Add (Variables|Default|Getguns) (LocalVariables|GetincomingGun)))
      (Utilities|Array|Add (Variables|Default|GetisJunk) (LocalVariables|GetisIncomingJunk))))
  (return (not (LocalVariables|GetinventoryFull)) _returnvalue))

(fn IsInventoryFull
  (Math|Integer|CompareInt (Utilities|Array|Length (Variables|Default|Getguns)) (Variables|Default|GetinventorySize)
    (:>
      (LocalVariables|SetreturnValue true :!label _label))
    (:==
      (goto _label))
    (:<
      (LocalVariables|SetreturnValue false)))
  (return (LocalVariables|GetreturnValue)))

(fn RemoveGunfromInventory
  (params (indexToRemove :type Integer :default 0))
  (bind _output_get (LocalVariables|Setindex indexToRemove))
  (Math|Integer|CompareInt _output_get (Utilities|Array|Length (Variables|Default|Getguns))
    (:>
      (LocalVariables|SetreturnValue false :!label _label))
    (:==
      (goto _label))
    (:<
      (LocalVariables|Setgun (Utilities|Array|Get(acopy) (Variables|Default|Getguns) (LocalVariables|Getindex)))
      (Utilities|Array|RemoveIndex (Variables|Default|Getguns) (LocalVariables|Getindex))
      (Utilities|Array|RemoveIndex (Variables|Default|GetisJunk) (LocalVariables|Getindex))))
  (return (LocalVariables|GetreturnValue) (LocalVariables|Getgun)))

(fn GetGunfromIndex
  (params (index :type Integer :default 0))
  (return (Utilities|Array|Get(acopy) (Variables|Default|Getguns) index) (Utilities|Array|Get(acopy) (Variables|Default|GetisJunk) index)))

(fn SetJunkbyIndex
  (params (index :type Integer :default 0) (isJunk :type Boolean :default false))
  (Utilities|Array|SetArrayElem (Variables|Default|GetisJunk) index isJunk))