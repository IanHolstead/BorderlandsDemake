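; Base class for loot pickups, with a sprite plus a beam and light styled from its rarity.
; Overlapping characters auto-use consumables not spawned in chests; other loot joins their pickup stack until overlap ends.
; Use gates health items on the collector's need, while holdUse skips that check.
; Pickup removes it from stacks, disables collision and physics, lerps the sprite to the collector via timeline, then calls OnPickedUp.
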(event Custom|holdUse
  (params (collectingActor :type Character%20Base%20Class%20Object%20Reference))
  ;[1 1 1] Gun is already added to backpack
  (Variables|Default|SetCollectingActor collectingActor)
  (CallFunction|PrepareforPickup)
  ;[1 1 1] Pickup animation
  (bind _pickup_movement (Timeline|Pickup PlayFromStart)
    (:Update
      (Transformation|SetWorldLocation (Variables|Default|GetLootSprite) (Math|Vector|Lerp(Vector) (Transformation|GetWorldLocation (Variables|Default|GetLootSprite)) (+ (Transformation|GetActorLocation (Variables|Default|GetCollectingActor)) "0,0.000000, 0") _pickup_movement) false))
    (:Finished
      (Default|CallOnPickedUp))))

(event EventUse
  (params (user :type Character%20Base%20Class%20Object%20Reference) (secondUse :type Boolean))
  (Variables|Default|SetCollectingActor user)
  (|checkifplayerneedhealth
    (:OutputPin
      (CallFunction|PrepareforPickup)
      ;[1 1 1] Pickup animation
      (bind _pickup_movement (Timeline|Pickup PlayFromStart)
        (:Update
          (Transformation|SetWorldLocation (Variables|Default|GetLootSprite) (Math|Vector|Lerp(Vector) (Transformation|GetWorldLocation (Variables|Default|GetLootSprite)) (+ (Transformation|GetActorLocation (Variables|Default|GetCollectingActor)) "0,0.000000, 0") _pickup_movement) false))
        (:Finished
          (Default|CallOnPickedUp))))))

(event EventBeginPlay)

(event EventActorBeginOverlap
  (params (OtherActor :type Actor%20Object%20Reference))
  ;[1 1 1] Think about this, some things seem to be missed
  ;[1 1 1] Do nothing if being picked up
  (if (Collision|GetActorEnableCollision)
    (bind _ascharacter_base_class (Utilities|Casting|CastToCharacterBaseClass OtherActor))
    (Variables|Default|SetCollectingActor _ascharacter_base_class)
    (bind _isconsumable (CallFunction|IsConsumable (Variables|Default|GetLootRarity)))
    (if (and _isconsumable (not (Variables|Default|GetspawnInChest)))
      (|checkifplayerneedhealth
        (:OutputPin
          (CallFunction|PrepareforPickup)
          ;[1 1 1] Pickup animation
          (bind _pickup_movement (Timeline|Pickup PlayFromStart)
            (:Update
              (Transformation|SetWorldLocation (Variables|Default|GetLootSprite) (Math|Vector|Lerp(Vector) (Transformation|GetWorldLocation (Variables|Default|GetLootSprite)) (+ (Transformation|GetActorLocation (Variables|Default|GetCollectingActor)) "0,0.000000, 0") _pickup_movement) false))
            (:Finished
              (Default|CallOnPickedUp)))))
      (else
        (Default|AddtoPickupStack (Variables|Default|GetCollectingActor) self)))))

(event EventTick
  (params (DeltaSeconds :type Float%20%28single-precision%29))
  ;[1 1 1] Set loot pointer location
  (if (not (Variables|Rendering|GetbHidden))
    (Transformation|SetWorldLocation (Variables|Default|GetLootRarityBeam) (- (Transformation|GetWorldLocation (Variables|Default|GetLightAttachementPoint)) "0,0.100000, 0") false)))

(event EventActorEndOverlap
  (params (OtherActor :type Actor%20Object%20Reference))
  ;[1 1 1] Do nothing if being picked up
  (if (Collision|GetActorEnableCollision)
    (bind _ascharacter_base_class (Utilities|Casting|CastToCharacterBaseClass OtherActor))
    (Default|RemovefromPickupStack _ascharacter_base_class self)))

(fn ConstructionScript
  (Rendering|Components|Sprite|SetSprite (Variables|Default|GetLootSprite) (Variables|Default|GetSpriteToUse))
  (bind (_lootsprite _lightcolour) (CallFunction|LootRarityLookup (Variables|Default|GetLootRarity)))
  (Rendering|Components|Sprite|SetSprite (Variables|Default|GetLootRarityBeam) _lootsprite)
  (Rendering|Components|Light|SetLightColor (Variables|Default|GetLootRarityLight) _lightcolour)
  (Transformation|SetWorldTransform (Variables|Default|GetLootRarityBeam) (Math|Transform|MakeTransform (Transformation|GetWorldLocation (Variables|Default|GetLightAttachementPoint))) false))

(fn PrepareforPickup
  (CallFunction|RemovefromPickupStacks (Variables|Default|GetSphereCollisionComponent) 0 0 self)
  (Collision|SetActorEnableCollision self false)
  (Physics|SetSimulatePhysics (Variables|Default|GetLootSprite) false))

(fn GetPointerLocation
  (return (+ (Transformation|GetWorldLocation (Variables|Default|GetLightAttachementPoint)) "0,1.000000,85.000000")))