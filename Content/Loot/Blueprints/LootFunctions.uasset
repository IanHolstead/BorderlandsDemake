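; Blueprint function library for loot presentation and classification, keyed on a loot rarity enum that spans weapon-style tiers, mission items, Eridium, health and money.
; LootRarityLookup switches on the rarity to return a matching light sprite and light colour.
; IsConsumable switches on the same enum and returns true only for Health and Money, leaving every other rarity at the default value.
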(fn LootRarityLookup
  (params (lootRarity :type LootRarity%20Enum :default "NewEnumerator0"))
  (switch Utilities|FlowControl|Switch|SwitchonLootRarity lootRarity
    (:NewEnumerator0
      (LocalVariables|SetreturnSprite "/Game/Loot/LightBeams/Sprites/white_light_Sprite.white_light_Sprite")
      (LocalVariables|SetreturnColour "(R=1.000000,G=1.000000,B=1.000000,A=1.000000)"))
    (:NewEnumerator1
      (LocalVariables|SetreturnSprite "/Game/Loot/LightBeams/Sprites/green_light_Sprite.green_light_Sprite")
      (LocalVariables|SetreturnColour "(R=0.016667,G=1.000000,B=0.000000,A=1.000000)"))
    (:NewEnumerator2
      (LocalVariables|SetreturnSprite "/Game/Loot/LightBeams/Sprites/blue_light_Sprite.blue_light_Sprite")
      (LocalVariables|SetreturnColour "(R=0.000000,G=0.000000,B=1.000000,A=1.000000)"))
    (:NewEnumerator3
      (LocalVariables|SetreturnSprite "/Game/Loot/LightBeams/Sprites/purple_light_Sprite.purple_light_Sprite")
      (LocalVariables|SetreturnColour "(R=0.400000,G=0.000000,B=1.000000,A=1.000000)"))
    (:NewEnumerator4
      (LocalVariables|SetreturnSprite "/Game/Loot/LightBeams/Sprites/etech_light_Sprite.etech_light_Sprite")
      (LocalVariables|SetreturnColour "(R=1.000000,G=0.000000,B=0.689979,A=1.000000)"))
    (:NewEnumerator5
      (LocalVariables|SetreturnSprite "/Game/Loot/LightBeams/Sprites/orange_light_Sprite.orange_light_Sprite")
      (LocalVariables|SetreturnColour "(R=1.000000,G=0.185217,B=0.000000,A=1.000000)"))
    (:NewEnumerator10
      (LocalVariables|SetreturnSprite "/Game/Loot/LightBeams/Sprites/mission_light_Sprite.mission_light_Sprite")
      (LocalVariables|SetreturnColour "(R=0.000000,G=1.000000,B=0.978464,A=1.000000)"))
    (:NewEnumerator8
      (LocalVariables|SetreturnSprite "/Game/Loot/LightBeams/Sprites/eridium_light_Sprite.eridium_light_Sprite")
      (LocalVariables|SetreturnColour "(R=0.856177,G=0.000000,B=1.000000,A=1.000000)"))
    (:NewEnumerator6
      (LocalVariables|SetreturnSprite "/Game/Loot/LightBeams/Sprites/health_light_Sprite.health_light_Sprite")
      (LocalVariables|SetreturnColour "(R=1.000000,G=0.000000,B=0.000000,A=1.000000)"))
    (:NewEnumerator7
      (LocalVariables|SetreturnSprite "/Game/Loot/LightBeams/Sprites/money_light_Sprite.money_light_Sprite")
      (LocalVariables|SetreturnColour "(R=1.000000,G=0.660102,B=0.019184,A=1.000000)")))
  (return (LocalVariables|GetreturnSprite) (LocalVariables|GetreturnColour)))

(fn IsConsumable
  (params (lootRarity :type LootRarity%20Enum :default "NewEnumerator0"))
  (switch Utilities|FlowControl|Switch|SwitchonLootRarity lootRarity
    (:NewEnumerator0
      _)
    (:NewEnumerator1
      _)
    (:NewEnumerator2
      _)
    (:NewEnumerator3
      _)
    (:NewEnumerator4
      _)
    (:NewEnumerator5
      _)
    (:NewEnumerator10
      _)
    (:NewEnumerator8
      _)
    (:NewEnumerator6
      (LocalVariables|SetreturnValue true :!label _label))
    (:NewEnumerator7
      (goto _label)))
  (return (LocalVariables|GetreturnValue)))