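; Health pickup actor that restores a quarter of the collecting actor's max health over time, then destroys itself.
; On BeginPlay it binds to its picked-up event; when used, it hides itself and plays a timeline.
; Each timeline update lerps toward the total and adds only the rounded difference from what was already given, so healing arrives gradually in whole increments.
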(event Custom|Event%20pickup%20used
  (Rendering|SetActorHiddenInGame true)
  (bind _maxhealth (Default|GetMaxHealth (Variables|Default|GetCollectingActor)))
  (Variables|Default|Sethealth (/ _maxhealth 4))
  (bind _health (Timeline|health%20timeline PlayFromStart)
    (:Update
      (Default|AddHealth (Variables|Default|GetCollectingActor) (- (Math|Float|Round (Math|Float|Lerp 0.0 (Math|Conversions|ToFloat(Integer) (Variables|Default|Gethealth)) _health)) (Variables|Default|GethealthAdded)))
      (Variables|Default|SethealthAdded (Math|Float|Round (Math|Float|Lerp 0.0 (Math|Conversions|ToFloat(Integer) (Variables|Default|Gethealth)) _health))))
    (:Finished
      (Actor|DestroyActor))))

(event EventBeginPlay
  (EventDispatchers|BindEventtoOnPickedUp (delegate Custom|Event%20pickup%20used)))

(fn ConstructionScript
  (|CallParentFunction))