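; Eridium loot pickup that grants the collecting actor Eridium currency.
; The construction script runs the parent's setup, then sets the pickup's value to a single Eridium.
; On BeginPlay it binds to the picked-up event, which adds that value to the collector and destroys the pickup.
; It also supplies the Eridium sound as its use sound.
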(event Custom|Pickup%20Grabbed
  (Default|AddEridium (Variables|Default|GetCollectingActor) (Variables|Default|GetEridiumValue))
  (Actor|DestroyActor))

(event EventBeginPlay
  (EventDispatchers|BindEventtoOnPickedUp (delegate Custom|Pickup%20Grabbed)))

(fn ConstructionScript
  (|CallParentFunction)
  (Variables|Default|SetEridiumValue 1))

(fn GetUseSound
  (return "/Game/Audio/Effects/eridium.eridium"))