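; Short-lived muzzle flash sprite for guns, tinted by the weapon's element.
; The construction script maps Element to a Paper2D sprite colour.
; Tick accumulates Age and, until it exceeds LifeSpan, sets a world transform from the owner's current gun location and PlayerDirection, with zero scale.
; The actor destroys itself once LifeSpan is exceeded or the owner is no longer holding a gun.
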(event EventBeginPlay)

(event EventTick
  (params (DeltaSeconds :type Float%20%28single-precision%29))
  (bind _owningactor (Variables|Default|GetOwningActor))
  (bind _output_get (Variables|Default|Setage (+ DeltaSeconds (Variables|Default|Getage))))
  (Math|Float|CompareFloat _output_get (Variables|Default|GetlifeSpan)
    (:>
      (Actor|DestroyActor :!label _label))
    (:==
      (bind (_isholdinggun _currentgun) (Default|GetCurrentGun _owningactor :!label _label_2))
      (if _isholdinggun
        (Transformation|SetWorldTransform (Math|Transform|MakeTransform (Transformation|GetWorldLocation _currentgun) (Variables|/Game/Characters/Blueprints/CharacterBaseClass.CharacterBaseClass_C|GetPlayerDirection _owningactor)) false)
        (else
          (goto _label))))
    (:<
      (goto _label_2))))

(fn ConstructionScript
  (switch Utilities|FlowControl|Switch|SwitchonElementalTypes (Variables|Default|Getelement)
    (:NewEnumerator4
      (LocalVariables|Setcolour "(R=1.000000,G=1.000000,B=1.000000,A=1.000000)"))
    (:NewEnumerator0
      (LocalVariables|Setcolour "(R=0.000000,G=0.123422,B=1.000000,A=1.000000)"))
    (:NewEnumerator1
      (LocalVariables|Setcolour "(R=1.000000,G=0.008761,B=0.000000,A=1.000000)"))
    (:NewEnumerator2
      (LocalVariables|Setcolour "(R=0.000000,G=1.000000,B=0.203581,A=1.000000)"))
    (:NewEnumerator3
      (LocalVariables|Setcolour "(R=1.000000,G=1.000000,B=1.000000,A=1.000000)"))
    (:NewEnumerator5
      (LocalVariables|Setcolour "(R=0.677428,G=0.000000,B=1.000000,A=1.000000)")))
  (Sprite|SetSpriteColor (Variables|Default|GetPaperSprite) (LocalVariables|Getcolour)))