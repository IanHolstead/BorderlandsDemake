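; Base gun loot class that hides itself when picked up and handles timed single or automatic firing, with bullet creation still a placeholder.
; Each shot plays a sound, adds fire-rate and recoil stacks, then waits on a delay before re-firing if automatic.
; Fire-rate stacks slow firing, while recoil stacks are only tracked here.
; Tick ages and expires both stacks while owned, otherwise running parent loot behavior.
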(event Custom|Shoot
  (if (not (Variables|Default|GetisWaiting))
    (Variables|Default|SetkeepShooting true)
    ;[1 1 1] create bullet here
    (Development|PrintString "bang!")
    (Class|GameplayStatics|PlaySoundAttached (Variables|Audio|GetshootSound) (Variables|Default|GetLootSprite))
    (CallFunction|AddDelayStack (+ (Variables|GunData|GetburstFireRounds) (Variables|GunData|GetshotsPerShot)))
    (bind _firerate (CallFunction|GetFireRate))
    (Variables|Default|SetisWaiting true)
    (Development|PrintString (Utilities|String|ToString(Float) _firerate))
    (Utilities|FlowControl|Delay (/ 1.0 _firerate))
    (Variables|Default|SettimeSinceFireRateStackChange 0.0)
    (Variables|Default|SettimeSinceRecoilStackChange 0.0)
    (Variables|Default|SetisWaiting false)
    (if (and (Variables|GunData|GetfullyAutomatic) (Variables|Default|GetkeepShooting))
      (CallFunction|Shoot))))

(event Custom|Stop%20Shooting
  (Variables|Default|SetkeepShooting false))

(event Custom|Pickup%20Grabbed
  (Rendering|SetActorHiddenInGame true)
  (Rendering|Components|Light|SetIntensity (Variables|Default|GetLootRarityLight) 0.0))

(event EventBeginPlay
  (EventDispatchers|BindEventtoOnPickedUp (delegate Custom|Pickup%20Grabbed)))

(event EventTick
  (params (DeltaSeconds :type Float%20%28single-precision%29))
  ;[1 1 1] Age gun if it has owner
  (bind _hasowner (CallFunction|DoesGunHaveOwner))
  (if _hasowner
    (CallFunction|AgeGun DeltaSeconds)
    (else
      (|CallParentFunction DeltaSeconds))))

(fn ConstructionScript
  (Variables|Default|SetLootRarity (Variables|GunData|Getrarity))
  (|CallParentFunction))

(fn AgeGun
  (params (Age :type Float%20%28single-precision%29 :default 0.0))
  (LocalVariables|SettimeToAge Age)
  (Utilities|AgeStacks (Variables|Default|GettimeSinceFireRateStackChange) (Variables|GunData|GetfireRateDelayDecay) (LocalVariables|Getindex) (Variables|GunData|GetcurentFireRateStack) (LocalVariables|GettimeToAge) (Variables|GunData|GetcurentFireRateStack)
    (:Completed
      (Utilities|AgeStacks (Variables|Default|GettimeSinceRecoilStackChange) (Variables|GunData|GetrecoilDecay) (LocalVariables|Getindex) (Variables|GunData|GetcurrentRecoilStack) (LocalVariables|GettimeToAge) (Variables|GunData|GetcurrentRecoilStack)
        (:Completed
          (Variables|Default|SettimeSinceFireRateStackChange (+ (LocalVariables|GettimeToAge) (Variables|Default|GettimeSinceFireRateStackChange)))
          (Variables|Default|SettimeSinceRecoilStackChange (+ (LocalVariables|GettimeToAge) (Variables|Default|GettimeSinceRecoilStackChange)))
          (if (not (and (Variables|GunData|GetfullyAutomatic) (Variables|Default|GetkeepShooting)))
            (bind _firerate (CallFunction|GetFireRate))
            (if (< (/ 1.0 _firerate) (Variables|Default|GettimeSinceFireRateStackChange))
              (Variables|Default|SettimeSinceFireRateStackChange 0.0)
              (Utilities|Array|RemoveIndex (Variables|GunData|GetcurentFireRateStack)))
            (if (< (Variables|GunData|GetrecoilDecay) (Variables|Default|GettimeSinceRecoilStackChange))
              (Variables|Default|SettimeSinceRecoilStackChange 0.0)
              (Utilities|Array|RemoveIndex (Variables|GunData|GetcurrentRecoilStack)))))))))

(fn GetFireRate
  (return (Math|Float|Max(Float) (- (Variables|GunData|GetfireRate) (* (Utilities|Array|Length (Variables|GunData|GetcurentFireRateStack)) (Variables|GunData|GetfireRateDelay))) 0.0001)))

(fn DoesGunHaveOwner
  (return (Utilities|IsValid (Variables|Default|Getcharacter))))

(fn AgeMuzzleFlash
  (params (timeToAge :type Float%20%28single-precision%29 :default 0.0))
  (bind _firerate (CallFunction|GetFireRate)))

(fn AddDelayStack
  (params (numberOfStacks :type Integer :default 0))
  (for _index (range 1 numberOfStacks)
    (Utilities|Array|Add (Variables|GunData|GetcurentFireRateStack) 0.0)
    (Utilities|Array|Add (Variables|GunData|GetcurrentRecoilStack) 0.0)))