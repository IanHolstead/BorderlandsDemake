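; Bullet projectile actor for guns, launched by a physics impulse on its BulletDecal at BeginPlay.
; Tick tracks distance from spawn and destroys it once attenuation reaches 100%.
; For player-owned hits on enemies, DamageBox hits roll accuracy, then crit, and scale damage by distance; misses destroy the bullet.
; Unfinished: ApplyDamage is disconnected, the elemental roll leads nowhere, and non-player hits on characters do nothing.
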(event OnComponentHit(DamageBox)
  (params (OtherActor :type Actor%20Object%20Reference) (OtherComp :type Primitive%20Component%20Object%20Reference) (NormalImpulse :type Vector :default "0, 0, 0") (Hit :type Hit%20Result%20Structure%20%28by%20ref%29))
  (bind _aspawn (Utilities|Casting|CastToPawn OtherActor))
  (Variables|Default|SetdamageReciever _aspawn)
  (if (Variables|Default|GetisOwnerCharacter)
    (Utilities|Casting|CastToEnemyBaseClass (Variables|Default|GetdamageReciever)
      (:then
        ;[1 1 1] does it hit?
        (Math|Float|CompareFloat (Variables|Default|Getaccuracy) (Math|Random|RandomFloatinRange 0.0 1e+02)
          (:>
            ;[1 1 1] Crits
            (if (Variables|Default|GetcanCrit) :!label _label
              (if true
                (Math|Float|CompareFloat (Variables|Default|GetCritChance) (Math|Random|RandomFloatinRange 0.0 1e+02)
                  (:>
                    (Variables|Default|Setdamage (Math|Float|Round (* (Variables|Default|Getdamage) (Variables|Default|GetcritMultiplier))) :!label _label_2))
                  (:==
                    (goto _label_2))
                  (:<
                    _))))
            (Variables|Default|Setdamage (Math|Float|Round (* (Variables|Default|Getdamage) (Math|Float|Clamp(Float) (/ (- 1e+02 (* (Variables|Default|GetattenuationPerMeter) (Variables|Default|GetdistanceTraveled))) 1e+02)))))
            (Math|Float|CompareFloat (Variables|Default|GetelementalChance) (Math|Random|RandomFloatinRange 0.0 1e+02)))
          (:==
            (goto _label))
          (:<
            (Actor|DestroyActor :!label _label_3))))
      (:CastFailed
        (goto _label_3)))
    (else
      (Utilities|Casting|CastToCharacterBaseClass (Variables|Default|GetdamageReciever)
        (:CastFailed
          (goto _label_3))))))

(event EventBeginPlay
  (Variables|Default|SetspawnLocation (Transformation|GetWorldLocation (Variables|Default|GetDamage%20Box)))
  (Physics|AddImpulse (Variables|Default|GetBullet%20Decal) (Variables|Default|Getvelocity) "None" false))

(event Collision|EventActorBeginOverlap
  (params (OtherActor :type Actor%20Object%20Reference)))

(event EventTick
  (params (DeltaSeconds :type Float%20%28single-precision%29))
  (bind _output_get (Variables|Default|SetdistanceTraveled (Math|Vector|VectorLength (- (Variables|Default|GetspawnLocation) (Transformation|GetWorldLocation (Variables|Default|GetDamage%20Box))))))
  (Math|Float|CompareFloat (* _output_get (Variables|Default|GetattenuationPerMeter)) 1e+02
    (:>
      _)
    (:==
      _))
  (Actor|DestroyActor))

(fn ConstructionScript)