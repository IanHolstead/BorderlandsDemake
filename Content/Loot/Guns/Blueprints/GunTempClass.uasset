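; Temporary gun class in the loot system that spawns bullets with type, element, crit and accuracy stats, supporting full-auto via a delayed, self-calling Shoot.
; Each shot adds timed fire-rate and recoil stacks, and fire-rate stacks lower the effective rate.
; While owned by a Character, Tick ages and expires those stacks through the AgeStacks macro; otherwise it runs parent Tick.
; Muzzle-flash aging is unfinished, and recoil stacks are only tracked here.
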(event Custom|Shoot
  (if (not (Variables|Default|GetisWaiting))
    (Variables|Default|SetkeepShooting true)
    (CallFunction|FireBullet)
    ;[1 1 1] fix
    (Audio|SpawnSoundAttached (Variables|Audio|GetshootSound) 0)
    (CallFunction|AddDelayStack (+ (Variables|GunData|GetburstFireRounds) (Variables|GunData|GetshotsPerShot)))
    (bind _firerate (CallFunction|GetFireRate))
    (Variables|Default|SetisWaiting true)
    (Development|PrintString (Utilities|String|ToString(Float) _firerate))
    (Utilities|FlowControl|Delay (/ 1.0 _firerate))
    (Variables|Default|SettimeSinceFireRateStackChange 0.0)
    (Variables|Default|SettimeSinceRecoilStackChange 0.0)
    (Variables|Default|SetisWaiting false)
    (if (and (Variables|GunData|GetfullyAutomatic) (Variables|Default|GetkeepShooting))
      (CallFunction|Shoot))))

(event Custom|Stop%20Shooting
  (Variables|Default|SetkeepShooting false))

(event EventBeginPlay)

(event EventTick
  (params (DeltaSeconds :type Float%20%28single-precision%29))
  ;[1 1 1] Age gun if it has owner
  (bind _hasowner (CallFunction|DoesGunHaveOwner))
  (if _hasowner
    (CallFunction|AgeGun DeltaSeconds)
    (else
      (|CallParentFunction DeltaSeconds))))

(fn ConstructionScript)

(fn AgeGun
  (params (Age :type Float%20%28single-precision%29 :default 0.0))
  (LocalVariables|SettimeToAge Age)
  (Utilities|AgeStacks (Variables|Default|GettimeSinceFireRateStackChange) (Variables|GunData|GetfireRateDelayDecay) (LocalVariables|Getindex) (Variables|GunData|GetcurentFireRateStack) (LocalVariables|GettimeToAge) (Variables|GunData|GetcurentFireRateStack)
    (:Completed
      (Utilities|AgeStacks (Variables|Default|GettimeSinceRecoilStackChange) (Variables|GunData|GetrecoilDecay) (LocalVariables|Getindex) (Variables|GunData|GetcurrentRecoilStack) (LocalVariables|GettimeToAge) (Variables|GunData|GetcurrentRecoilStack)
        (:Completed
          (Variables|Default|SettimeSinceFireRateStackChange (+ (LocalVariables|GettimeToAge) (Variables|Default|GettimeSinceFireRateStackChange)))
          (Variables|Default|SettimeSinceRecoilStackChange (+ (LocalVariables|GettimeToAge) (Variables|Default|GettimeSinceRecoilStackChange)))
          (if (not (and (Variables|GunData|GetfullyAutomatic) (Variables|Default|GetkeepShooting)))
            (bind _firerate (CallFunction|GetFireRate))
            (if (< (/ 1.0 _firerate) (Variables|Default|GettimeSinceFireRateStackChange))
              (Variables|Default|SettimeSinceFireRateStackChange 0.0)
              (Utilities|Array|RemoveIndex (Variables|GunData|GetcurentFireRateStack)))
            (if (< (Variables|GunData|GetrecoilDecay) (Variables|Default|GettimeSinceRecoilStackChange))
              (Variables|Default|SettimeSinceRecoilStackChange 0.0)
              (Utilities|Array|RemoveIndex (Variables|GunData|GetcurrentRecoilStack)))))))))

(fn GetFireRate
  (return (Math|Float|Max(Float) (- (Variables|GunData|GetfireRate) (* (Utilities|Array|Length (Variables|GunData|GetcurentFireRateStack)) (Variables|GunData|GetfireRateDelay))) 0.0001)))

(fn DoesGunHaveOwner
  (return (Utilities|IsValid (Variables|Default|Getcharacter))))

(fn AgeMuzzleFlash
  (params (timeToAge :type Float%20%28single-precision%29 :default 0.0))
  (bind _firerate (CallFunction|GetFireRate)))

(fn AddDelayStack
  (params (numberOfStacks :type Integer :default 0))
  (for _index (range 1 numberOfStacks)
    (Utilities|Array|Add (Variables|GunData|GetcurentFireRateStack) 0.0)
    (Utilities|Array|Add (Variables|GunData|GetcurrentRecoilStack) 0.0)))

(fn FireBullet
  (bind _character (Variables|Default|Getcharacter))
  (bind _returnvalue (Game|SpawnActorfromClass "/Game/Loot/Guns/Blueprints/Bullet.Bullet_C" (Transformation|GetWorldTransform (Variables|Default|GetGunBarrelExitPoint)) "Undefined" self (Variables|GunData|GetgunType) (Variables|GunData|Getelement) (* (Math|Vector|RotateVector (Math|Vector|MakeVector 1.0 0.0 0.0) (Transformation|GetActorRotation (Variables|Default|Getcharacter))) 5e+03) (Variables|GunData|GetelementalChance) (Variables|GunData|GetelementalDamage) (Variables|GunData|GetcanCrit) (Variables|GunData|GetcritChance) (Variables|GunData|GetcritMultiplier) (Variables|GunData|GetbulletAttenuationPerMeter) (Variables|GunData|Getaccuracy) _character _character))
  (Class|PrimitiveComponent|SetConstraintMode (Variables|/Game/Loot/Guns/Blueprints/Bullet.Bullet_C|GetBullet%20Decal _returnvalue) "XZPlane"))