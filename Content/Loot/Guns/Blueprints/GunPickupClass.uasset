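; A gun loot pickup Blueprint that configures itself from a Gun data value and hides when collected.
; The construction script copies the gun's sprite and rarity into inherited pickup variables, then runs the parent construction script.
; On BeginPlay it binds to the OnPickedUp event, which hides the actor and turns off its rarity light by zeroing intensity.
; Tick only calls the parent implementation.
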(event Custom|Pickup%20Grabbed
  (Rendering|SetActorHiddenInGame true)
  (Rendering|Components|Light|SetIntensity (Variables|Default|GetLootRarityLight) 0.0))

(event EventBeginPlay
  (EventDispatchers|BindEventtoOnPickedUp (delegate Custom|Pickup%20Grabbed)))

(event EventTick
  (params (DeltaSeconds :type Float%20%28single-precision%29))
  (|CallParentFunction DeltaSeconds))

(fn ConstructionScript
  (Variables|Default|SetSpriteToUse (Variables|/Game/Loot/Guns/Blueprints/GunBaseClass.GunBaseClass_C|GetgunSprite (Variables|Default|Getgun)))
  (Variables|Default|SetLootRarity (Variables|/Game/Loot/Guns/Blueprints/GunBaseClass.GunBaseClass_C|Getrarity (Variables|Default|Getgun)))
  (|CallParentFunction))